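; Game instance that manages front-end menus, multiplayer sessions and network error reporting.
; A save check opens the main menu, or the options menu with a welcome message when no settings save exists.
; Show events create and display widgets, caching all but the server browser.
; Hosting creates a session and opens Lobby as a listen server; session, network and travel failures feed a shared error dialog.
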(event `SaveGameCheck`
  (bind _returnvalue (`GameplayStatics.DoesSaveGameExist` (`self.PlayerSettingsSave`)))
  (if _returnvalue
    (`self.ShowMainMenu`)
    (set `self.CreatedSaveFile?` true)
    (else
      (`self.ShowOptionsMenu`)
      (set `PlayerController.bShowMouseCursor` true (`GameplayStatics.GetPlayerController` 0)))))

(event `self.HandleNetworkError`
  (params (FailureType :type "ENetworkFailure Enum" :default "NetDriverAlreadyExists") (bIsServer :type Boolean))
  (if bIsServer
    _
    (else
      _))
  (`self.DesplayErrorMessage` (`self.NetErrorToString` FailureType)))

(event `ShowMainMenu`
  (bind _returnvalue (`GameplayStatics.GetPlayerController` 0))
  (`/Engine/EditorBlueprintResources/StandardMacros.IsValid` (`self.MainMenuWB`)
    (:`Is Valid`
      _)
    (:`Is Not Valid`
      (bind _returnvalue_2 (`|CreateWidget` "/Game/UI/MainMenu/WB_MainMenu.WB_MainMenu_C" _returnvalue))
      (set `self.MainMenuWB` _returnvalue_2)))
  (`UserWidget.AddToViewport` (`self.MainMenuWB`) 0)
  (set `PlayerController.bShowMouseCursor` true _returnvalue))

(event `ShowLoadingScreen`
  (`/Engine/EditorBlueprintResources/StandardMacros.IsValid` (`self.LoadingScreenWB`)
    (:`Is Valid`
      _)
    (:`Is Not Valid`
      (bind _returnvalue (`|CreateWidget` "/Game/UI/AllLevels/WB_LoadingScreen.WB_LoadingScreen_C" (`GameplayStatics.GetPlayerController` 0)))
      (set `self.LoadingScreenWB` _returnvalue)))
  (`UserWidget.AddToViewport` (`self.LoadingScreenWB`) 0))

(event `self.HandleTravelError`
  (params (FailureType :type "ETravelFailure Enum" :default "NoLevel"))
  (`self.DesplayErrorMessage` (`self.TravelErrorToString` FailureType)))

(event `LaunchLobby`
  (params (NumerOfPlayers :type Integer) (`EnableLan?` :type Boolean) (ServerName :type Text))
  (set `self.Max Player` NumerOfPlayers)
  (set `self.Server Name` ServerName)
  (`self.ShowLoadingScreen`)
  (`CreateSessionCallbackProxy.CreateSession` (`GameplayStatics.GetPlayerController` 0) (`self.Max Player`) `EnableLan?`
    (:`OnSuccess`
      (`GameplayStatics.OpenLevel` "Lobby" true "listen"))
    (:`OnFailure`
      (`self.DesplayErrorMessage` "Faild to create Session"))))

(event `ShowHostMenu`
  (`/Engine/EditorBlueprintResources/StandardMacros.IsValid` (`self.HostMenuWB`)
    (:`Is Valid`
      _)
    (:`Is Not Valid`
      (bind _returnvalue (`|CreateWidget` "/Game/UI/MainMenu/WB_HostMenu.WB_HostMenu_C" (`GameplayStatics.GetPlayerController` 0)))
      (set `self.HostMenuWB` _returnvalue)))
  (`UserWidget.AddToViewport` (`self.HostMenuWB`) 0))

(event `DestroySessionCaller`
  (params (PlaterController :type "PlayerController Object Reference"))
  (`DestroySessionCallbackProxy.DestroySession` PlaterController))

(event `ShowServerMenu`
  (bind _returnvalue (`|CreateWidget` "/Game/UI/MainMenu/WB_ServerBrowser.WB_ServerBrowser_C" (`GameplayStatics.GetPlayerController` 0)))
  (`UserWidget.AddToViewport` _returnvalue 0))

(event `JoinServer`
  (params (SessionToJoin :type "BlueprintSessionResult Structure"))
  (`self.ShowLoadingScreen`)
  (`JoinSessionCallbackProxy.JoinSession` (`GameplayStatics.GetPlayerController` 0) SessionToJoin
    (:`OnFailure`
      (`self.DesplayErrorMessage` "Faild to join session"))))

(event `ShowOptionsMenu`
  (`/Engine/EditorBlueprintResources/StandardMacros.IsValid` (`self.OptionsMenu`)
    (:`Is Valid`
      _)
    (:`Is Not Valid`
      (bind _returnvalue (`|CreateWidget` "/Game/UI/MainMenu/OptionsMenu.OptionsMenu_C" (`GameplayStatics.GetPlayerController` 0)))
      (set `self.OptionsMenu` _returnvalue)))
  (`UserWidget.AddToViewport` (`self.OptionsMenu`) 0)
  (if (not (`self.CreatedSaveFile?`))
    (set `/Game/UI/MainMenu/OptionsMenu.WellcomeMessageVis` "Visible" (`self.OptionsMenu`))))

(fn `NetErrorToString`
  (params (FailureType :type "ENetworkFailure Enum" :default "NetDriverAlreadyExists"))
  (returns (OutStirng :type String))
  (switch `ENetworkFailure` FailureType
    (:`NetDriverAlreadyExists`
      (set `self.ErrorString` "Error: Lost Connection to Host" :!label _label))
    (:`NetDriverCreateFailure`
      (goto _label))
    (:`NetDriverListenFailure`
      (goto _label))
    (:`ConnectionLost`
      (goto _label))
    (:`ConnectionTimeout`
      (set `self.ErrorString` "Error: Connection Time Out"))
    (:`FailureReceived`
      (goto _label))
    (:`OutdatedClient`
      (goto _label))
    (:`OutdatedServer`
      (goto _label))
    (:`PendingConnectionFailure`
      (goto _label))
    (:`NetGuidMismatch`
      (goto _label))
    (:`NetChecksumMismatch`
      (goto _label)))
  (return (`self.ErrorString`)))

(fn `OnRep_Max Player`)

(fn `TravelErrorToString`
  (params (FailureType :type "ETravelFailure Enum" :default "NoLevel"))
  (returns (OutString :type String))
  (return (`KismetStringLibrary.Concat_StrStr` "Error: Failed to Travel" (`|GetEnumeratorNameAsString` FailureType))))
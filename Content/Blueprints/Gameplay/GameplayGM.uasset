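; Multiplayer gameplay game mode that handles respawning, match results and logout.
; It tracks controllers as they swap, and respawning replaces a controller's existing pawn with a new character at a random PlayerStart.
; Logout asks the game instance to destroy that player's session.
; RestartGame prints the winner and calls Win on it and Lose on other player pawns, without reloading the level.
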(event `self.K2_OnSwapPlayerControllers`
  (params (OldPC :type "PlayerController Object Reference") (NewPC :type "PlayerController Object Reference"))
  (bind _allplayercontrollers (`self.AllPlayerControllers`))
  (`KismetArrayLibrary.Array_Add` _allplayercontrollers NewPC)
  (`KismetArrayLibrary.Array_RemoveItem` _allplayercontrollers OldPC))

(event `RespawnPlayer`
  (params (PlayerController :type "PlayerController Object Reference") (PlayerCharacter :type "Character Class Reference"))
  (bind _returnvalue (`Controller.K2_GetPawn` PlayerController))
  (bind _spawnpoints (`self.SpawnPoints`))
  (bind _outactors (`GameplayStatics.GetAllActorsOfClass` "/Script/Engine.PlayerStart"))
  (set `self.SpawnPoints` _outactors)
  (`/Engine/EditorBlueprintResources/StandardMacros.IsValid` _returnvalue
    (:`Is Valid`
      (`self.K2_DestroyActor` _returnvalue)
      (bind _returnvalue_2 (`|SpawnActorFromClass` PlayerCharacter (`self.GetTransform` (`|GetArrayItem` _spawnpoints (`KismetMathLibrary.RandomIntegerInRange` 0 (- (`KismetArrayLibrary.Array_Length` _spawnpoints) 1)))) "Undefined" "MultiplyWithRoot" null null))
      (`Controller.Possess` PlayerController _returnvalue_2))))

(event `self.K2_OnLogout`
  (params (ExitingController :type "Controller Object Reference"))
  (bind _asgameplay_pc (cast `/Game/Blueprints/Gameplay/GameplayPC` ExitingController))
  (`/Game/Blueprints/AllLevels/GameInfoInstance.DestroySessionCaller` (cast `/Game/Blueprints/AllLevels/GameInfoInstance` (`GameplayStatics.GetGameInstance`) :!pure true) _asgameplay_pc))

(event `RestartGame`
  (params (WinningPlayer :type "/Game/Blueprints/Characters/0_Base Object Reference"))
  (`KismetSystemLibrary.PrintString` (`KismetSystemLibrary.GetDisplayName` WinningPlayer))
  (`/Game/Blueprints/Characters/0_Base.Win` WinningPlayer)
  (bind _returnvalue (`self.GetNumPlayers`))
  (for _index (range _returnvalue)
    (bind _as0_base (cast `/Game/Blueprints/Characters/0_Base` (`GameplayStatics.GetPlayerPawn` _index)))
    (if (!= _as0_base WinningPlayer)
      (`/Game/Blueprints/Characters/0_Base.Lose` _as0_base))))

(fn `UserConstructionScript`)
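; Gameplay player controller that applies the player's saved character choice when play begins.
; On the local controller, BeginPlay clears all widgets, loads PlayerSettings from the save slot and hands it to PassCharacterInfoToServer.
; That event stores the settings and asks GameplayGM to respawn the player as the saved character.
; The respawn call passes only the character, and its guard checks player controller 0 rather than this controller.
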(event `self.ReceiveBeginPlay`
  (if (`self.IsLocalController`)
    (`WidgetLayoutLibrary.RemoveAllWidgets`)
    (`self.LoadGame`)
    (`self.PassCharacterInfoToServer` (`self.PlayerSettings`))))

(event `PassCharacterInfoToServer`
  (params (PlayerSettingsInfo :type "/Game/Blueprints/AllLevels/PlayerInfo Structure"))
  (set `self.PlayerSettings` PlayerSettingsInfo)
  (bind _asgameplay_gm (cast `/Game/Blueprints/Gameplay/GameplayGM` (`GameplayStatics.GetGameMode`)))
  (cast `/Game/Blueprints/Gameplay/GameplayPC` (`GameplayStatics.GetPlayerController` 0))
  (`/Game/Blueprints/Gameplay/GameplayGM.RespawnPlayer` _asgameplay_gm null (`.MyPlayerCharacter_13_7A965628429B0183768812B878C9B7E3` (break `/Game/Blueprints/AllLevels/PlayerInfo` (`self.PlayerSettings`)))))

(fn `LoadGame`
  (bind _returnvalue (`GameplayStatics.LoadGameFromSlot` (`self.PlayerSettingsSave`)))
  (bind _asplayer_sacve_game (cast `/Game/Blueprints/AllLevels/PlayerSacveGame` _returnvalue))
  (set `self.PlayerSettings` (`/Game/Blueprints/AllLevels/PlayerSacveGame.S_PlayerInfo` _asplayer_sacve_game)))

(fn `UserConstructionScript`)
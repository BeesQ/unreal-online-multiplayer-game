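; Lobby game mode that registers joining players, sets up their lobby UI from the game instance's server settings and possesses a pawn at a random PlayerStart.
; EveryoneUpdate rebroadcasts player counts, info and available characters to each LobbyPC; map setting changes are pushed likewise.
; LaunchTheGame server-travels to one of two arenas by MapID after a delay.
; Kick-list and character-swap events are empty, and both readiness branches set CanWeStart true.
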(event `self.K2_PostLogin`
  (params (NewPlayer :type "PlayerController Object Reference"))
  (`/Engine/EditorBlueprintResources/ActorMacros.Switch Has Authority`
    (:`Authority`
      (`KismetArrayLibrary.Array_Add` (`self.AllPlayerControllers`) NewPlayer)
      (bind _outactors (`GameplayStatics.GetAllActorsOfClass` "/Script/Engine.PlayerStart"))
      (set `self.SpawnPoints` _outactors)
      (bind _asgame_info_instance (cast `/Game/Blueprints/AllLevels/GameInfoInstance` (`GameplayStatics.GetGameInstance`)))
      (set `self.Server Name` (`/Game/Blueprints/AllLevels/GameInfoInstance.Server Name` _asgame_info_instance))
      (set `self.Max Player` (`/Game/Blueprints/AllLevels/GameInfoInstance.Max Player` _asgame_info_instance))
      (bind _aslobby_pc (cast `/Game/Blueprints/Lobby/LobbyPC` NewPlayer))
      (`/Game/Blueprints/Lobby/LobbyPC.InialSetup` _aslobby_pc)
      (`/Game/Blueprints/Lobby/LobbyPC.SetupLobbyMenu` _aslobby_pc (`self.Server Name`))
      (`/Game/Blueprints/Lobby/LobbyPC.UpdateLobbySettings` _aslobby_pc (`self.GM Map Image`) (`self.Map Name`) (`self.Map Time`))
      (`self.RespawnPlayer` NewPlayer))))

(event `RespawnPlayer`
  (params (PlayerController :type "PlayerController Object Reference"))
  (bind _returnvalue (`Controller.K2_GetPawn` PlayerController))
  (bind _spawnpoints (`self.SpawnPoints`))
  (`/Engine/EditorBlueprintResources/StandardMacros.IsValid` _returnvalue
    (:`Is Valid`
      (`self.K2_DestroyActor` _returnvalue))
    (:`Is Not Valid`
      _))
  (bind _returnvalue_2 (`|SpawnActorFromClass` "/Game/Blueprints/Characters/0_Base.0_Base_C" (`self.GetTransform` (`|GetArrayItem` _spawnpoints (`KismetMathLibrary.RandomIntegerInRange` 0 (- (`KismetArrayLibrary.Array_Length` _spawnpoints) 1)))) "Undefined" "MultiplyWithRoot" null null))
  (`Controller.Possess` PlayerController _returnvalue_2)
  (`self.EveryoneUpdate`))

(event `EveryoneUpdate`
  (bind _allplayercontrollers (`self.AllPlayerControllers`))
  (bind _connectedplayers (`self.ConnectedPlayers`))
  (bind _connectedplayers_2 (`self.ConnectedPlayers`))
  (bind _output_get (set `self.CurrentPlayers` (`KismetArrayLibrary.Array_Length` (`self.AllPlayerControllers`))))
  (if (> _output_get 0)
    (`KismetArrayLibrary.Array_Clear` _connectedplayers_2)
    (for _array_element _allplayercontrollers
      (bind _aslobby_pc (cast `/Game/Blueprints/Lobby/LobbyPC` _array_element))
      (`KismetArrayLibrary.Array_Add` _connectedplayers (`/Game/Blueprints/Lobby/LobbyPC.PlayerSettings` _aslobby_pc))
      (`/Game/Blueprints/Lobby/LobbyPC.UpdateNumberOfPlayers` _aslobby_pc (`self.CurrentPlayers`) (`self.Max Player`)))
    (for _array_element_2 _allplayercontrollers
      (bind _aslobby_pc_2 (cast `/Game/Blueprints/Lobby/LobbyPC` _array_element_2))
      (`/Game/Blueprints/Lobby/LobbyPC.AddPlayerInfo` _aslobby_pc_2 _connectedplayers)
      (`/Game/Blueprints/Lobby/LobbyPC.UpdateAvailableCharacters` _aslobby_pc_2 (`self.Available Characters`))
      (`self.AddToKickList`))
    (for _array_element_3 _connectedplayers_2 :!label _label
      (if (== (`.MyPlayerCharacter_13_7A965628429B0183768812B878C9B7E3` (break `/Game/Blueprints/AllLevels/PlayerInfo` _array_element_3)) "/Game/Blueprints/Characters/0_Base.0_Base_C")
        (set `self.CanWeStart?` true)
        (else
          (set `self.CanWeStart?` true))))))

(event `AddToKickList`)

(event `ServerUpdaterGameSettings`
  (params (MapImage :type "Texture2D Object Reference") (MapName :type Text) (MapTime :type Text) (MapID :type Integer))
  (set `self.GM Map Image` MapImage)
  (set `self.Map Name` MapName)
  (set `self.Map Time` MapTime)
  (set `self.Map ID` MapID)
  (for _array_element (`self.AllPlayerControllers`)
    (bind _aslobby_pc (cast `/Game/Blueprints/Lobby/LobbyPC` _array_element))
    (`/Game/Blueprints/Lobby/LobbyPC.UpdateLobbySettings` _aslobby_pc (`self.GM Map Image`) (`self.Map Name`) (`self.Map Time`))))

(event `CannotStartGame`
  (goto _label :!via `Break`))

(event `LaunchTheGame`
  (bind _returnvalue (`GameplayStatics.GetPlayerController` 0))
  (switch `int` (`self.Map ID`)
    (:`0`
      (`KismetSystemLibrary.Delay` 5.0)
      (`KismetSystemLibrary.ExecuteConsoleCommand` "servertravel  Arena" _returnvalue))
    (:`1`
      (`KismetSystemLibrary.Delay` 5.0)
      (`KismetSystemLibrary.ExecuteConsoleCommand` "servertravel  Arena1" _returnvalue))))

(event `SwapCharacter`
  (params (PlayerController :type "PlayerController Object Reference") (CharacterClass :type "Character Class Reference") (ChangedStatus :type Boolean)))

(fn `UserConstructionScript`)
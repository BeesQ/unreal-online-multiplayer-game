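; Player controller for the multiplayer lobby that manages each player's profile, lobby menu and loading screen.
; Initial setup syncs name and image with a save slot, resets the character to base, then has LobbyGM swap it and update everyone.
; Events feed the player list, player count and map details into the menu widget, and T toggles its panels.
; Being kicked opens the main menu; both that and EndPlay destroy the session.
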(event `InialSetup`
  (`self.SeveGameCheck`)
  (`self.CallUpdate` (`self.PlayerSettings`)))

(event `SetupLobbyMenu`
  (params (ServerName :type Text))
  (set `self.bShowMouseCursor` true)
  (bind _returnvalue (`|CreateWidget` "/Game/UI/Lobby/WB_LobbyMenu.WB_LobbyMenu_C" null ServerName))
  (bind _output_get (set `self.LobbyMenuWB` _returnvalue))
  (`UserWidget.AddToViewport` _output_get 0)
  (`WidgetBlueprintLibrary.SetInputMode_GameAndUIEx` self _output_get))

(event `CallUpdate`
  (params (PlayerInfo :type "/Game/Blueprints/AllLevels/PlayerInfo Structure") (`ChangeStatus?` :type Boolean))
  (bind _aslobby_gm (cast `/Game/Blueprints/Lobby/LobbyGM` (`GameplayStatics.GetGameMode`) :!pure true))
  (set `self.PlayerSettings` PlayerInfo)
  (`/Game/Blueprints/Lobby/LobbyGM.SwapCharacter` _aslobby_gm self (`.MyPlayerCharacter_13_7A965628429B0183768812B878C9B7E3` (break `/Game/Blueprints/AllLevels/PlayerInfo` (`self.PlayerSettings`))) `ChangeStatus?`)
  (`/Game/Blueprints/Lobby/LobbyGM.EveryoneUpdate` _aslobby_gm))

(event `AddPlayerInfo`
  (params (ConnectedPlayerInfo :type "Array of /Game/Blueprints/AllLevels/PlayerInfo Structure"))
  (bind _lobbymenuwb (`self.LobbyMenuWB`))
  (set `self.AllConnecterdPlayers` ConnectedPlayerInfo)
  (`/Engine/EditorBlueprintResources/StandardMacros.IsValid` _lobbymenuwb
    (:`Is Valid`
      (`/Game/UI/Lobby/WB_LobbyMenu.ClearPlayerList` _lobbymenuwb)
      (for _array_element (`self.AllConnecterdPlayers`)
        (`/Game/UI/Lobby/WB_LobbyMenu.UpdatePlayerWindow` (`self.LobbyMenuWB`) _array_element)))))

(event `UpdateLobbySettings`
  (params (MapImage :type "Texture2D Object Reference") (MapName :type Text) (MapTime :type Text))
  (bind _lobbymenuwb (`self.LobbyMenuWB`))
  (set `/Game/UI/Lobby/WB_LobbyMenu.MapImage` MapImage _lobbymenuwb)
  (set `/Game/UI/Lobby/WB_LobbyMenu.MapName` MapName _lobbymenuwb)
  (set `/Game/UI/Lobby/WB_LobbyMenu.MapTime` MapTime _lobbymenuwb))

(event `ShowLoadingScreen`
  (`Widget.RemoveFromParent` (`self.LobbyMenuWB`))
  (bind _returnvalue (`|CreateWidget` "/Game/UI/AllLevels/WB_LoadingScreen.WB_LoadingScreen_C" self))
  (`UserWidget.AddToViewport` _returnvalue 0))

(event `UpdateNumberOfPlayers`
  (params (CurrentPlayers :type Integer) (MaxPlayers :type Integer))
  (bind _lobbymenuwb (`self.LobbyMenuWB`))
  (`/Engine/EditorBlueprintResources/StandardMacros.IsValid` _lobbymenuwb
    (:`Is Valid`
      (set `/Game/UI/Lobby/WB_LobbyMenu.PlayersDisplay` (`|FormatText` "{CurrentPlayers} of {MaxPlayers}" CurrentPlayers MaxPlayers) _lobbymenuwb))))

(event `UpdateAvailableCharacters`
  (params (AvailableCharacters :type "Array of Boolean")))

(event `self.ReceiveEndPlay`
  (params (EndPlayReason :type "EEndPlayReason Enum" :default "Destroyed"))
  (`DestroySessionCallbackProxy.DestroySession` self :!label _label))

(event `Kicked`
  (`GameplayStatics.OpenLevel` "MeinMennu")
  (goto _label))

(event `Key|T`
  (params (Key :type "Key Structure"))
  (bind _playerlist (`/Game/UI/Lobby/WB_LobbyMenu.PlayerList` (`self.LobbyMenuWB`)))
  (:`Pressed`
    (`/Engine/EditorBlueprintResources/StandardMacros.FlipFlop`
      (:`A`
        (`Widget.SetVisibility` _playerlist "Hidden")
        (`Widget.SetVisibility` (`/Game/UI/Lobby/WB_LobbyMenu.LobbySettings` (`self.LobbyMenuWB`)) "Hidden"))
      (:`B`
        (`Widget.SetVisibility` _playerlist "Visible")
        (`Widget.SetVisibility` (`/Game/UI/Lobby/WB_LobbyMenu.LobbySettings` (`self.LobbyMenuWB`)) "Visible")))))

(fn `LoadGame`
  (bind _returnvalue (`GameplayStatics.LoadGameFromSlot` (`self.PlayerSettingsSave`)))
  (bind _asplayer_sacve_game (cast `/Game/Blueprints/AllLevels/PlayerSacveGame` _returnvalue))
  (bind (_myplayername _myplayerimage) (break `/Game/Blueprints/AllLevels/PlayerInfo` (`/Game/Blueprints/AllLevels/PlayerSacveGame.S_PlayerInfo` _asplayer_sacve_game)))
  (setmembers `/Game/Blueprints/AllLevels/PlayerInfo` :`StructRef` (`self.PlayerSettings`) :`MyPlayerName` _myplayername :`MyPlayerImage` _myplayerimage :`MyPlayerCharacter` "/Game/Blueprints/Characters/0_Base.0_Base_C" :`MyPlayerCharacterImage` null))

(fn `SaveGame`
  (bind _playersacvegameref (`self.PlayerSacveGameRef`))
  (`/Engine/EditorBlueprintResources/StandardMacros.IsValid` (`self.PlayerSacveGameRef`)
    (:`Is Valid`
      _)
    (:`Is Not Valid`
      (bind _returnvalue (`GameplayStatics.CreateSaveGameObject` "/Game/Blueprints/AllLevels/PlayerSacveGame.PlayerSacveGame_C"))
      (bind _asplayer_sacve_game (cast `/Game/Blueprints/AllLevels/PlayerSacveGame` _returnvalue))
      (set `self.PlayerSacveGameRef` _asplayer_sacve_game)))
  (set `/Game/Blueprints/AllLevels/PlayerSacveGame.S_PlayerInfo` (`self.PlayerSettings`) _playersacvegameref)
  (`GameplayStatics.SaveGameToSlot` _playersacvegameref (`self.PlayerSettingsSave`)))

(fn `SeveGameCheck`
  (bind _returnvalue (`GameplayStatics.DoesSaveGameExist` (`self.PlayerSettingsSave`)))
  (if _returnvalue
    (`self.LoadGame`)
    (`self.SaveGame`)
    (else
      (`self.SaveGame`))))

(fn `UserConstructionScript`)